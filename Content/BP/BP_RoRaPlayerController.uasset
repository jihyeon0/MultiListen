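; Player controller Blueprint for RoRa, apparently meant to relay chat messages between the HUD and the game mode, but currently inactive.
; BeginPlay and the OnSendMsgToServer event (noted as a server RPC) have empty bodies.
; Disconnected leftover nodes show the earlier design: delayed binding to WBP_RoRaHUD, forwarding messages to BP_RoRaGameMode, and updating HUD text on local controllers.
; None of that leftover logic runs.
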(event `self.ReceiveBeginPlay`)

(event `OnSendMsgToServer`
  (params (Message :type String))
  ; 클라 -> 서버
  ;; 게임모드에게 메세지를 넘겨줌
  ;;; 서버 RPC로 변경해줬음
)

(fn `UserConstructionScript`)